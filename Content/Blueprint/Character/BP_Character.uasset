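; Top-down player character Blueprint that handles movement-mode input and camera zoom and shake.
; Walk, sprint and aim inputs set flags and call ChangeMovementState, and Tick prints the resulting state for debugging.
; Construction configures the camera boom, while the mouse wheel zooms it within height limits through a looping timer that slides arm length in increments.
; The F key triggers a camera shake, and the instant-step SlideCamera zoom remains unused.
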(event EventTick
  (params (DeltaSeconds :type Float%20%28single-precision%29))
  (Development|PrintString (Utilities|String|EnumtoString (Variables|Default|GetMovementState)) true true "(R=0.000000,G=0.660000,B=1.000000,A=1.000000)" 0.0))

(event Input|ActionEvents|InputActionMovementModeChangeSprint
  (params (Key :type Key%20Structure))
  (:Pressed
    (Variables|Default|SetSprintRunEnabled true)
    (Class|TPSCharacter|ChangeMovementState :!label _label))
  (:Released
    (Variables|Default|SetSprintRunEnabled false)
    (goto _label)))

(event Input|ActionEvents|InputActionMovementModeChangeWalk
  (params (Key :type Key%20Structure))
  (:Pressed
    (Variables|Default|SetWalkEnabled true)
    (Class|TPSCharacter|ChangeMovementState :!label _label))
  (:Released
    (Variables|Default|SetWalkEnabled false)
    (goto _label)))

(event Input|ActionEvents|InputActionRightMouse
  (params (Key :type Key%20Structure))
  (:Pressed
    (Variables|Default|SetAimEnabled true)
    (Class|TPSCharacter|ChangeMovementState :!label _label))
  (:Released
    (Variables|Default|SetAimEnabled false)
    (goto _label)))

(event Input|AxisEvents|InputAxisMouseWheel
  (params (AxisValue :type Float%20%28single-precision%29))
  (CallFunction|CameraSlideSmooth AxisValue))

(event Input|KeyboardEvents|F
  (params (Key :type Key%20Structure))
  (:Pressed
    (CallFunction|ShakeCamera)))

(fn ConstructionScript
  (bind _cameraboom (Variables|Default|GetCameraBoom))
  (Variables|/Script/Engine.SpringArmComponent|SetTargetArmLength _cameraboom (Variables|Camera|GetMinHieghtCamera))
  (Transformation|SetRelativeRotation _cameraboom (Variables|Camera|GetRotatorCamera) false false)
  (Variables|/Script/Engine.SpringArmComponent|SetbEnableCameraLag _cameraboom (Variables|Camera|GetFlow))
  (Variables|/Script/Engine.SpringArmComponent|SetCameraLagSpeed _cameraboom (Variables|Camera|GetCoffSmooth)))

(fn ShakeCamera
  (Camera|PlayWorldCameraShake "/Game/Blueprint/Game/BP_ShakeCamera.BP_ShakeCamera_C" (Transformation|GetWorldLocation (Variables|Default|GetTopDownCameraComponent)) 0.0 3e+01))

(fn CameraSlideSmooth
  (params (Value :type Float%20%28single-precision%29))
  (bind _cameraboom (Variables|Default|GetCameraBoom))
  (bind _heightchangecameradistance (Variables|Camera|GetHeightChangeCameraDistance))
  (bind _targetarmlength (Variables|/Script/Engine.SpringArmComponent|GetTargetArmLength _cameraboom))
  (if (Variables|Slide|GetSlideDone)
    (if (!= Value 0.0)
      (if (< Value 0.0)
        (if (>= (Variables|Camera|GetMaxHieghtCamera) (+ _targetarmlength _heightchangecameradistance))
          (Variables|Slide|SetSlideUp true)
          (Variables|Slide|SetSlideDone false :!label _label)
          (bind _returnvalue (Utilities|Time|SetTimerbyFunctionName 0 "CameraSlideSmoothTick" (Variables|Slide|GetTimer) true))
          (Variables|Slide|SetSlideTimer _returnvalue))
        (elif (<= (Variables|Camera|GetMinHieghtCamera) (- _targetarmlength _heightchangecameradistance))
          (Variables|Slide|SetSlideUp false)
          (goto _label))))))

(fn CameraSlideSmoothTick
  (bind _hieghtcamerachangeslidedistance (Variables|Slide|GetHieghtCameraChangeSlideDistance))
  (bind _cameraboom (Variables|Default|GetCameraBoom))
  (bind _output_get (Variables|Slide|SetCurrentSlideDistance (+ (Variables|Slide|GetCurrentSlideDistance) _hieghtcamerachangeslidedistance)))
  (Variables|/Script/Engine.SpringArmComponent|SetTargetArmLength _cameraboom (select (Variables|Slide|GetSlideUp) (+ (Variables|/Script/Engine.SpringArmComponent|GetTargetArmLength _cameraboom) _hieghtcamerachangeslidedistance) (- (Variables|/Script/Engine.SpringArmComponent|GetTargetArmLength _cameraboom) _hieghtcamerachangeslidedistance)))
  (if (>= _output_get (Variables|Camera|GetHeightChangeCameraDistance))
    (Variables|Slide|SetCurrentSlideDistance 0.0)
    (Variables|Slide|SetSlideDone true)
    (Utilities|Time|ClearandInvalidateTimerbyHandle (Variables|Slide|GetSlideTimer))))

(fn SlideCamera
  (params (NewParam :type Float%20%28single-precision%29))
  (bind _heightchangecameradistance (Variables|Camera|GetHeightChangeCameraDistance))
  (bind _cameraboom (Variables|Default|GetCameraBoom))
  (if (!= NewParam 0.0)
    (if (< NewParam 0.0)
      (if (>= (Variables|Camera|GetMaxHieghtCamera) (+ (Variables|/Script/Engine.SpringArmComponent|GetTargetArmLength (Variables|Default|GetCameraBoom)) _heightchangecameradistance))
        (Variables|/Script/Engine.SpringArmComponent|SetTargetArmLength _cameraboom (+ (Variables|/Script/Engine.SpringArmComponent|GetTargetArmLength (Variables|Default|GetCameraBoom)) _heightchangecameradistance)))
      (elif (<= (Variables|Camera|GetMinHieghtCamera) (- (Variables|/Script/Engine.SpringArmComponent|GetTargetArmLength (Variables|Default|GetCameraBoom)) _heightchangecameradistance))
        (Variables|/Script/Engine.SpringArmComponent|SetTargetArmLength _cameraboom (- (Variables|/Script/Engine.SpringArmComponent|GetTargetArmLength (Variables|Default|GetCameraBoom)) _heightchangecameradistance))))))